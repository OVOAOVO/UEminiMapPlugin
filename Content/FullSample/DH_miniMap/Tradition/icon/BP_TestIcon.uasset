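; BP_TestIcon is a map icon actor for a minimap sample, marking its world position on the minimap.
; Its construction script sets the billboard sprite from the icon texture.
; UpdateIconLocation passes the 2D offset from the first player pawn to a valid minimap icon, and GetMapIconData returns location, texture, size and the actor itself.
; The event graph's events, including ZoomMap, are empty.
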(event `self.ReceiveBeginPlay`)

(event `self.ReceiveTick`
  (params (DeltaSeconds :type "Float (single-precision)")))

(event `self.ZoomMap`
  (params (`In/Out` :type Boolean)))

(fn `GetMapIconData`
  (returns (location :type "Vector Structure") (icon :type "Texture2D Object Reference") (`icon size` :type "Vector2D Structure") (`world actor` :type "Actor Object Reference"))
  (bind _icon_component_minimap (`self.icon_Component_miniMap`))
  (return (`self.K2_GetActorLocation`) (`/TraditionalRPGminiMap/FullSample/DH_miniMap/Tradition/icon/icon_Component_miniMap.icon_Texture` _icon_component_minimap) (`/TraditionalRPGminiMap/FullSample/DH_miniMap/Tradition/icon/icon_Component_miniMap.miniMap_icon_Size` _icon_component_minimap) self))

(fn `Update Icon Location`
  (bind _icon_minimap (`self.icon_miniMap`)
    (:`then`
      (`/TraditionalRPGminiMap/FullSample/DH_miniMap/Tradition/icon/icon_miniMap_widget.Update Icon Location` _icon_minimap (`KismetMathLibrary.Conv_VectorToVector2D` (- (`self.K2_GetActorLocation`) (`self.K2_GetActorLocation` (`GameplayStatics.GetPlayerPawn` 0))))))
    (:`else`)))

(fn `UserConstructionScript`
  (`BillboardComponent.SetSprite` (`self.Billboard`) (`self.icon_Texture`)))