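; Minimap HUD that manages the on-screen minimap, its fog of war and a toggleable, zoomable full key map.
; BeginPlay creates the minimap and a separate fog widget layered above it, then clears the fog render target.
; Tick writes player location to a Material Parameter Collection and draws the fog material into that target.
; Opening the key map spawns icons for BPI_MapItem actors and switches input to cursor-enabled Game and UI.
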(event `self.ReceiveBeginPlay`
  (bind _returnvalue (`|CreateWidget` "/TraditionalRPGminiMap/FullSample/DH_miniMap/Tradition/Tradition_miniMap_Widget.Tradition_miniMap_Widget_C"))
  (`UserWidget.AddToViewport` _returnvalue 0)
  (set `self.miniMap` _returnvalue)
  (`KismetRenderingLibrary.ClearRenderTarget2D` "/TraditionalRPGminiMap/FullSample/DH_miniMap/Tradition/warFog/maskFog.maskFog")
  ;[1 1 1] miniMapFog: 写在这里是因为地图先创建，icon后创建，半透明混合不正确
  (bind _returnvalue_2 (`|CreateWidget` "/TraditionalRPGminiMap/FullSample/DH_miniMap/Tradition/warFog/miniMapFogWidget.miniMapFogWidget_C"))
  (`UserWidget.AddToViewport` _returnvalue_2 1))

(event `self.ReceiveTick`
  (params (DeltaSeconds :type "Float (single-precision)"))
  (`KismetMaterialLibrary.SetVectorParameterValue` "/TraditionalRPGminiMap/FullSample/DH_miniMap/Tradition/miniMap_parameterCorrection.miniMap_parameterCorrection" "Player Location" (`KismetMathLibrary.Conv_VectorToLinearColor` (`self.K2_GetActorLocation` (`GameplayStatics.GetPlayerCharacter` 0))))
  (`self.miniMapFogDraw`))

(event `M Key Map`
  (params (Condition :type Boolean))
  (bind _returnvalue (`GameplayStatics.GetPlayerController` 0))
  (bind _mapicon_array (`self.mapIcon_Array`))
  (if Condition
    (`self.KeyMap`
      (:`then`
        _)
      (:`else`
        (bind _returnvalue_2 (`|CreateWidget` "/TraditionalRPGminiMap/FullSample/DH_miniMap/Tradition/M_key_map/M_key_Map.M_key_Map_C"))
        (set `self.KeyMap` _returnvalue_2)))
    (`UserWidget.AddToViewport` (`self.KeyMap`) 0)
    (bind _outactors (`GameplayStatics.GetAllActorsWithInterface` "/TraditionalRPGminiMap/FullSample/DH_miniMap/Tradition/M_key_map/BPI_MapItem.BPI_MapItem_C"))
    (for _array_element _outactors
      (bind _returnvalue_3 (`|CreateWidget` "/TraditionalRPGminiMap/FullSample/DH_miniMap/Tradition/M_key_map/M_key_icon.M_key_icon_C"))
      (bind (_location _icon _icon_size _world_actor) (message `/TraditionalRPGminiMap/FullSample/DH_miniMap/Tradition/M_key_map/BPI_MapItem.GetMapIconData` _array_element))
      (`/TraditionalRPGminiMap/FullSample/DH_miniMap/Tradition/M_key_map/M_key_icon.Init icon` _returnvalue_3 _icon _world_actor)
      (`/TraditionalRPGminiMap/FullSample/DH_miniMap/Tradition/M_key_map/M_key_Map.Add Icon` (`self.KeyMap`) _returnvalue_3 (`KismetMathLibrary.Conv_VectorToVector2D` _location) _icon_size)
      (`KismetArrayLibrary.Array_Add` (`self.mapIcon_Array`) _returnvalue_3))
    (`WidgetBlueprintLibrary.SetInputMode_GameAndUIEx` _returnvalue null)
    (set `PlayerController.bShowMouseCursor` true _returnvalue)
    (`/TraditionalRPGminiMap/FullSample/DH_miniMap/Tradition/M_key_map/M_key_Map.Set Arrow Position` (`self.KeyMap`))
    (else
      (bind _keymap (`self.KeyMap`)
        (:`then`
          (if (`Widget.IsInViewport` _keymap)
            (`Widget.RemoveFromParent` _keymap)
            (for _array_element_2 _mapicon_array
              (bind _asm_key_icon (cast `/TraditionalRPGminiMap/FullSample/DH_miniMap/Tradition/M_key_map/M_key_icon` _array_element_2))
              (bind _hoveredbutton (`/TraditionalRPGminiMap/FullSample/DH_miniMap/Tradition/M_key_map/M_key_icon.HoveredButton` _asm_key_icon)
                (:`then`
                  (`Widget.RemoveFromParent` _hoveredbutton)
                  (`Widget.RemoveFromParent` _array_element_2)
                  (`WidgetBlueprintLibrary.SetInputMode_GameOnly` _returnvalue)
                  (set `PlayerController.bShowMouseCursor` false _returnvalue))
                (:`else`)))
            (`KismetArrayLibrary.Array_Clear` _mapicon_array)))
        (:`else`)))))

(event `ZoomKeyMap`
  (params (`Input/Out` :type Boolean))
  (bind _keymap (`self.KeyMap`)
    (:`then`
      (`/TraditionalRPGminiMap/FullSample/DH_miniMap/Tradition/M_key_map/M_key_Map.Zoom` _keymap `Input/Out`)
      (`/TraditionalRPGminiMap/FullSample/DH_miniMap/Tradition/M_key_map/M_key_Map.Set Arrow Position` (`self.KeyMap`)))
    (:`else`)))

(event `De select All Map Icons`
  (for _array_element (`self.mapIcon_Array`)
    (`/TraditionalRPGminiMap/FullSample/DH_miniMap/Tradition/M_key_map/M_key_icon.DeSelect` _array_element)))

(event `miniMapFogDraw`
  (`KismetRenderingLibrary.DrawMaterialToRenderTarget` "/TraditionalRPGminiMap/FullSample/DH_miniMap/Tradition/warFog/maskFog.maskFog" (`self.MaterialToRenderTarget`)))

(fn `GetMapIconData`
  (returns (location :type "Vector Structure") (icon :type "Texture2D Object Reference") (`icon size` :type "Vector2D Structure"))
  (return (0.0 0.0 0.0) null (0.0 0.0)))

(fn `UserConstructionScript`)